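; Cannon effect actor that fires a Niagara effect while the left mouse button is held.
; Mouse press and release toggle a count between one and zero, which Tick writes to the FXCannon spawn-count user parameter every frame.
; Tick also sets the Sphere's world rotation from the player camera rotation, scaled up by a constant multiplier.
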(event EventBeginPlay)

(event Collision|EventActorBeginOverlap
  (params (OtherActor :type Actor%20Object%20Reference)))

(event EventTick
  (params (DeltaSeconds :type Float%20%28single-precision%29))
  (Transformation|SetWorldRotation (Variables|Default|GetSphere) (* (Camera|GetCameraRotation (Game|GetPlayerCameraManager 0)) 7.0) false false)
  (Class|NiagaraComponent|SetVariableInt (Variables|Default|GetFX_Cannon) "User.Spawn Count" (Variables|Default|GetCount)))

(event Input|MouseEvents|LeftMouseButton
  (params (Key :type Key%20Structure :default "None"))
  (:Pressed
    (Variables|Default|SetCount 1))
  (:Released
    (Variables|Default|SetCount 0)))

(fn ConstructionScript)